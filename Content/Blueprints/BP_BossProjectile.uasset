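; BP_BossProjectile is a boss projectile that damages the player character on overlap and expires after a short lifetime counted on Tick.
; Collision overlaps ignore anything that is not BP_PlayerCharacter, then deal damage through BPI_Damageable, falling back to the player's HealthComponent.
; A successful hit spawns a particle effect and destroys the projectile.
; An unconnected loop over damageable components never runs.
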(event OnComponentBeginOverlap(Collision)
  (params (OverlappedComponent :type Primitive%20Component%20Object%20Reference) (OtherActor :type Actor%20Object%20Reference) (OtherComp :type Primitive%20Component%20Object%20Reference) (OtherBodyIndex :type Integer) (bFromSweep :type Boolean) (SweepResult :type Hit%20Result%20Structure%20%28by%20ref%29))
  (bind _returnvalue (Actor|GetComponentbyClass OtherActor "/Script/Project.HealthComponent"))
  (bind _collision (Variables|Default|GetCollision))
  ;[1 1 1] Check if we hit an actor and not just a wall
  (Utilities|IsValid OtherActor
    (:Is%20Valid
      (Utilities|Casting|CastToBP_PlayerCharacter OtherActor)
      ;[1 1 1] BPI_Damageable
      (if (Utilities|DoesObjectImplementInterface OtherActor "/Game/Blueprints/BPI_Damageable.BPI_Damageable_C")
        (Class|BPIDamageable|DoDamage(Message) OtherActor (Variables|Default|GetDamageAmount))
        (else
          ;[1 1 1] Check if it has Health
          (Utilities|IsValid _returnvalue
            (:Is%20Valid
              (Class|HealthComponent|DoDamage _returnvalue (Variables|Default|GetDamageAmount))))))
      (Effects|SpawnEmitteratLocation "/Game/Particles/P_BossProjectileParticle.P_BossProjectileParticle" (Transformation|GetWorldLocation _collision) (Transformation|GetWorldRotation _collision))
      (Actor|DestroyActor))))

(event EventBeginPlay
  (Variables|Default|SetLifeSpan 4.0)
  (Variables|Default|SetDamageAmount 1e+01))

(event Collision|EventActorBeginOverlap
  (params (OtherActor :type Actor%20Object%20Reference)))

(event EventTick
  (params (DeltaSeconds :type Float%20%28single-precision%29))
  ;[1 1 1] Destroy bullet after its been alive for too long
  (bind _output_get (Variables|Default|SetTimeAlive (+ DeltaSeconds (Variables|Default|GetTimeAlive))))
  (if (> _output_get (Variables|Default|GetLifeSpan))
    (Actor|DestroyActor)))

(fn ConstructionScript)