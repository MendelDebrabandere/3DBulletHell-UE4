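; Player character that fights with a gun and a sword, and respawns through BP_MyGameMode after death.
; BeginPlay spawns and attaches both weapons and creates the HUD; fire and timed sword-swing inputs are blocked once Health reports death.
; Tick tilts the gun socket with spring arm pitch and uses a downward trace to shrink the capsule while airborne for jumping over bullets.
; Death disables movement, then destroys character and weapons after a delay.
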(event OnDamage(Health)
  (params (DamageAmount :type Float%20%28single-precision%29))
  (Audio|PlaySoundatLocation "/Game/PlayerAssets/TakeDamage.TakeDamage" (Transformation|GetWorldLocation (Variables|Default|GetCapsuleComponent)) "0, 0, 0" 1.0 1.0 0.0 0 0 0))

(event OnDeath(Health)
  ;[1 1 1] Dissable character
  (Pawn|Components|CharacterMovement|DisableMovement (Variables|Character|GetCharacterMovement))
  (Default|FirePrimary (Variables|Default|GetCurrentWeapon) false)
  (Utilities|FlowControl|Delay 2.7)
  ;[1 1 1] Respawn
  (bind _asbp_my_game_mode (Utilities|Casting|CastToBP_MyGameMode (Game|GetGameMode))
    (:then
      (Default|RespawnPlayer _asbp_my_game_mode))
    (:CastFailed
      _))
  (Actor|DestroyActor (Variables|Default|GetCurrentWeapon)))

(event Custom|PrimaryFire
  (params (IsStart :type Boolean))
  ;[1 1 1] Shoot gun
  (if (not (Class|HealthComponent|IsDead (Variables|Default|GetHealth)))
    (bind _currentweapon (Variables|Default|GetCurrentWeapon)
      (:then
        (Default|FirePrimary _currentweapon IsStart))
      (:else))))

(event EventBeginPlay
  (bind _gun_socket (Variables|Default|GetGun%20socket))
  (bind _sword_socket (Variables|Default|GetSword%20Socket))
  (|CallParentFunction)
  (Utilities|FlowControl|Sequence
    (:then_0
      ;[1 1 1] Spawn sword
      (bind _returnvalue (Game|SpawnActorfromClass "/Game/Blueprints/BP_Sword.BP_Sword_C" (Transformation|GetWorldTransform _sword_socket) "Undefined" 0 0))
      (bind _output_get (Variables|Default|SetSword _returnvalue))
      (Transformation|AttachComponentToComponent _output_get _sword_socket "None" "SnapToTarget" "SnapToTarget" "SnapToTarget" true))
    (:then_1
      ;[1 1 1] Spawn gun
      (bind _returnvalue_2 (Game|SpawnActorfromClass "/Game/Blueprints/BP_BaseWeapon.BP_BaseWeapon_C" (Transformation|GetWorldTransform _gun_socket) "Undefined" 0 0))
      (bind _output_get_2 (Variables|Default|SetCurrentWeapon _returnvalue_2))
      (Transformation|AttachComponentToComponent _output_get_2 _gun_socket "None" "SnapToTarget" "SnapToTarget" "KeepRelative" true))
    (:then_2
      ;[1 1 1] Creating HUD
      (bind _returnvalue_3 (UserInterface|CreateWidget "/Game/Blueprints/BPW_GameHud.BPW_GameHud_C"))
      (UserInterface|Viewport|AddtoViewport _returnvalue_3 0))))

(event Collision|EventActorBeginOverlap
  (params (OtherActor :type Actor%20Object%20Reference)))

(event EventTick
  (params (DeltaSeconds :type Float%20%28single-precision%29))
  (bind _capsulecomponent (Variables|Default|GetCapsuleComponent))
  (bind _capsulecomponent_2 (Variables|Default|GetCapsuleComponent))
  (bind _returnvalue (Transformation|GetWorldLocation _capsulecomponent))
  ;[1 1 1] Make hitbox smaller when jumping to jump over the bullets
  (bind _returnvalue_2 (Collision|LineTraceByChannel _returnvalue (- _returnvalue "0, 0,91.000000") "TraceTypeQuery1" false 0 "None"))
  (if _returnvalue_2
    (Components|Capsule|SetCapsuleSize _capsulecomponent_2 34.0 88.0 true)
    (else
      (Components|Capsule|SetCapsuleSize _capsulecomponent_2 34.0 1e+01 true)))
  (Transformation|SetRelativeRotation (Variables|Default|GetGun%20socket) (Math|Rotator|MakeRotator 0.0 (+ (.Pitch (Math|Rotator|BreakRotator (Class|SpringArmComponent|GetTargetRotation (Variables|Default|GetSpringArm)))) 15.0) 9e+01) false false))

(event Input|ActionEvents|InputActionSwordAttack
  (params (Key :type Key%20Structure :default "None"))
  ;[1 1 1] Sword attack
  (:Pressed
    (if (not (Class|HealthComponent|IsDead (Variables|Default|GetHealth)))
      (Utilities|FlowControl|DoOnce false :!label _label
        (:Completed
          (Variables|/Game/Blueprints/BP_Sword.BP_Sword_C|SetIsSwinging (Variables|Default|GetSword) true)
          (Variables|/Game/Blueprints/BP_Sword.BP_Sword_C|SetHasHitThisSwing (Variables|Default|GetSword) false)
          (Animation|PlayAnimMontage "/Game/PlayerAssets/Animations/GreatSwordPack/AnimMontage.AnimMontage" 1.0 "None")
          (Audio|PlaySoundatLocation "/Game/PlayerAssets/Sword/SwingSword.SwingSword" (Transformation|GetWorldLocation (Variables|Default|GetCapsuleComponent)) "0, 0, 0" 1.0 1.0 0.0 0 0 0)
          (Utilities|FlowControl|Delay 0.6)
          (Variables|/Game/Blueprints/BP_Sword.BP_Sword_C|SetIsSwinging (Variables|Default|GetSword) false)
          (goto _label Reset))))))

(fn ConstructionScript
  (|CallParentFunction))