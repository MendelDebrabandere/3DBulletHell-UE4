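; Sword weapon actor that deals melee damage when its collision component overlaps another actor during a swing.
; It ignores the player character and allows only one hit attempt per swing through a flag.
; Damage goes through the BPI_Damageable interface, falling back to the target's HealthComponent.
; A successful hit spawns an impact particle at the sword's spawn point and a hit sound at the player pawn.
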(event OnComponentBeginOverlap(collision)
  (params (OverlappedComponent :type Primitive%20Component%20Object%20Reference) (OtherActor :type Actor%20Object%20Reference) (OtherComp :type Primitive%20Component%20Object%20Reference) (OtherBodyIndex :type Integer) (bFromSweep :type Boolean) (SweepResult :type Hit%20Result%20Structure%20%28by%20ref%29))
  (bind _returnvalue (Actor|GetComponentbyClass OtherActor "/Script/Project.HealthComponent"))
  (bind _particlespawnlocation (Variables|Default|GetParticleSpawnLocation))
  ;[1 1 1] Check if we hit an actor and not just a wall
  (Utilities|IsValid OtherActor
    (:Is%20Valid
      (if (Variables|Default|GetIsSwinging)
        ;[1 1 1] Cant be hitting yourself
        (Utilities|Casting|CastToBP_PlayerCharacter OtherActor
          (:CastFailed
            (if (not (Variables|Default|GetHasHitThisSwing))
              (Variables|Default|SetHasHitThisSwing true)
              ;[1 1 1] BPI_Damageable
              (if (Utilities|DoesObjectImplementInterface OtherActor "/Game/Blueprints/BPI_Damageable.BPI_Damageable_C")
                (Variables|Default|SetHasHitThisSwing true)
                (Class|BPIDamageable|DoDamage(Message) OtherActor (Variables|Default|GetDamageAmount))
                (else
                  ;[1 1 1] Check if it has Health
                  (Utilities|IsValid _returnvalue
                    (:Is%20Valid
                      (Variables|Default|SetHasHitThisSwing true)
                      (Class|HealthComponent|DoDamage _returnvalue (Variables|Default|GetDamageAmount))))))
              (Effects|SpawnEmitteratLocation "/Game/Particles/P_ParticleSwordImpact.P_ParticleSwordImpact" (Transformation|GetSocketLocation _particlespawnlocation "None") (Transformation|GetWorldRotation _particlespawnlocation))
              (Audio|SpawnSoundatLocation "/Game/PlayerAssets/Sword/SwordHit.SwordHit" (Transformation|GetActorLocation (Game|Player|GetPlayerPawn 0)) "0, 0, 0" 1.0 1.0 0.0 0 0))))))))

(event EventBeginPlay)

(event Collision|EventActorBeginOverlap
  (params (OtherActor :type Actor%20Object%20Reference)))

(event EventTick
  (params (DeltaSeconds :type Float%20%28single-precision%29)))

(fn ConstructionScript)