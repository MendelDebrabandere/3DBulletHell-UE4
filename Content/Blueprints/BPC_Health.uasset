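; BPC_Health is a Blueprint component that tracks health, resetting it to maximum on BeginPlay or through ResetHealth.
; DoDamage calls TookDamage before changing health, then subtracts the amount, clamped between zero and MaxHealth, and returns whether health is depleted.
; It compares against the cached previous health so OnDeath fires only when that call brings health to zero.
; Helper functions expose the health fraction and dead state.
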(event Custom|ResetHealth
  (Variables|Health|SetCurrentHealth (Variables|Health|GetMaxHealth)))

(event EventBeginPlay
  (CallFunction|ResetHealth))

(event EventTick
  (params (DeltaSeconds :type Float%20%28single-precision%29)))

(fn GetHealthPercentage
  (return (/ (Variables|Health|GetCurrentHealth) (Variables|Health|GetMaxHealth))))

(fn IsDead
  (return (== (CallFunction|GetHealthPercentage) 0.0)))

(fn DoDamage
  (params (Amount :type Float%20%28single-precision%29))
  (bind _isdead (CallFunction|IsDead))
  (Default|CallTookDamage)
  ;[1 1 1] Cache original health
  (LocalVariables|SetOriginalHealth (Variables|Health|GetCurrentHealth))
  (bind _output_get (Variables|Health|SetCurrentHealth (Math|Float|Clamp(Float) (- (Variables|Health|GetCurrentHealth) Amount) 0.0 (Variables|Health|GetMaxHealth))))
  ;[1 1 1] Did this call make the health 0?
  (if (and _isdead (> (LocalVariables|GetOriginalHealth) _output_get))
    (Default|CallOnDeath))
  (return _isdead))