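; Boss actor that runs a four-phase bullet-pattern fight keyed to health quarters and explodes on death.
; Tick drives timers for each phase's attacks, escalating from projectile rings through aimed shots to AOE fans, bouncing balls and spirals.
; Later phases open with a laugh, player-facing projectile arcs and a pause.
; Phases 3 and 4 are events to allow delayed loops, and player aiming is computed from world origin, ignoring boss position.
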(event OnDeath(Health)
  (bind _returnvalue (Game|Player|GetPlayerPawn 0))
  (bind _returnvalue_2 (Transformation|GetActorLocation _returnvalue))
  ;[1 1 1] Death
  (Effects|SpawnEmitteratLocation "/Game/StarterContent/Particles/P_Explosion.P_Explosion" (+ (Transformation|GetActorLocation) "0.000000,0.000000,300.000000") "0, 0, 0" "15.000000,15.000000,15.000000")
  (Audio|PlaySoundatLocation "/Game/StarterContent/Audio/Explosion01.Explosion01" _returnvalue_2 "0, 0, 0" 1.0 1.0 0.0 0 0 0)
  (Audio|PlaySoundatLocation "/Game/BossAssets/GameCompletion.GameCompletion" _returnvalue_2 "0, 0, 0" 1.0 1.0 0.0 0 0 0)
  (Actor|DestroyActor))

(event Custom|Phase%204
  (bind _rotator (CallFunction|GetRotationTowardsPlayer))
  (bind _defaultsceneroot (Variables|Default|GetDefaultSceneRoot))
  (bind _returnvalue (Transformation|GetWorldLocation _defaultsceneroot))
  ;[1 1 1] This phase could not be in a function because it has a delay
  ;[1 1 1] Wait 2 sec after phase change
  (if (Variables|Default|GetHasWaitedPhase4)
    (Utilities|FlowControl|Sequence
      (:then_0
        ;[1 1 1] Time attacks
        (if (> (Variables|Default|GetTotalTime) (Variables|Phase3|GetSeconsBetweenAttacksPhase3))
          (Variables|Default|SetTotalTime 0.0)
          ;[1 1 1] Set Vector directions
          (Variables|Phase3|SetAOE_Direction0 (* (Math|Vector|RotateVector "1.000000,0.000000,0.000000" _rotator) 1000))
          (Variables|Phase3|SetAOE_Direction1 (* (Math|Vector|RotateVector "0.866025,0.500000,0.000000" _rotator) 1000))
          (Variables|Phase3|SetAOE_Direction2 (* (Math|Vector|RotateVector "0.866025,-0.500000,0.000000" _rotator) 1000))
          (bind _index (Utilities|ForLoopwithDelay 1 4 0.5)
            (:LoopBody
              ;[1 1 1] Spawn 3 AOE attacks
              (Game|SpawnActorfromClass "/Game/Blueprints/BP_AOE_Attack.BP_AOE_Attack_C" (Math|Conversions|ToTransform(Vector) (+ (* (Variables|Phase3|GetAOE_Direction0) _index) _returnvalue)) "Undefined" 0 0)
              (Game|SpawnActorfromClass "/Game/Blueprints/BP_AOE_Attack.BP_AOE_Attack_C" (Math|Conversions|ToTransform(Vector) (+ (* (Variables|Phase3|GetAOE_Direction1) _index) _returnvalue)) "Undefined" 0 0)
              (Game|SpawnActorfromClass "/Game/Blueprints/BP_AOE_Attack.BP_AOE_Attack_C" (Math|Conversions|ToTransform(Vector) (+ (* (Variables|Phase3|GetAOE_Direction2) _index) _returnvalue)) "Undefined" 0 0)))))
      (:then_1
        ;[1 1 1] Time attacks
        (if (> (Variables|Default|GetTotalTime2) (Variables|Phase4|GetSecondsBetweenAttacksPhase4))
          (Variables|Default|SetTotalTime2 0.0)
          ;[1 1 1] Increment Rotator
          (Variables|Phase4|SetDirection0 (Math|Rotator|CombineRotators (Variables|Phase4|GetDirection0) (Variables|Phase4|GetDirectionIncrement)))
          ;[1 1 1] Spawn the bullets in a spiraling pattern
          (for _index_2 (range 0 7)
            (Game|SpawnActorfromClass "/Game/Blueprints/BP_BossProjectile.BP_BossProjectile_C" (Math|Transform|MakeTransform (+ (Transformation|GetActorLocation) "0.000000, 0,100.000000") (Math|Rotator|CombineRotators (Math|Rotator|MakeRotator 0.0 0.0 (* _index_2 45.0)) (Variables|Phase4|GetDirection0))) "Undefined" 0 0))))
      (:then_2
        ;[1 1 1] Time attacks
        (if (> (Variables|Phase4|GetTotalTime3) (Variables|Phase3|GetSecondsBetweenAttacksPhase3,2))
          (Variables|Phase4|SetTotalTime3 0.0)
          ;[1 1 1] Spawn bouncing bullets
          (for _index_3 (range 0 35)
            (bind _returnvalue_2 (Game|SpawnActorfromClass "/Game/Blueprints/BP_BossProjectile.BP_BossProjectile_C" (Math|Transform|MakeTransform (+ (Transformation|GetActorLocation) "0.000000, 0,100.000000") (Math|Rotator|MakeRotator 0.0 0.0 (Math|Conversions|ToFloat(Integer) (* _index_3 10)))) "Undefined" 0 0))
            (Variables|/Script/Engine.ProjectileMovementComponent|SetProjectileGravityScale (Variables|/Game/Blueprints/BP_BossProjectile.BP_BossProjectile_C|GetProjectileMovement _returnvalue_2) 1.0)
            (Game|Components|ProjectileMovement|SetVelocityinLocalSpace (Variables|/Game/Blueprints/BP_BossProjectile.BP_BossProjectile_C|GetProjectileMovement _returnvalue_2) (Math|Vector|MakeVector (.x (Variables|/Script/Engine.MovementComponent|GetVelocity (Variables|/Game/Blueprints/BP_BossProjectile.BP_BossProjectile_C|GetProjectileMovement _returnvalue_2))) (.y (Variables|/Script/Engine.MovementComponent|GetVelocity (Variables|/Game/Blueprints/BP_BossProjectile.BP_BossProjectile_C|GetProjectileMovement _returnvalue_2))) 1e+03))
            (Variables|/Script/Engine.ProjectileMovementComponent|SetbShouldBounce (Variables|/Game/Blueprints/BP_BossProjectile.BP_BossProjectile_C|GetProjectileMovement _returnvalue_2) true)
            (Collision|SetCollisionResponsetoChannel (Variables|/Game/Blueprints/BP_BossProjectile.BP_BossProjectile_C|GetCollision _returnvalue_2) "ECC_WorldStatic" "ECR_Block"))
          (Audio|SpawnSoundatLocation "/Game/BossAssets/BallSpawn.BallSpawn" "0, 0,100.000000" "0, 0, 0" 1.0 1.0 0.0 0 0))))
    (else
      (bind _output_get (Variables|Default|SetTotalTime (+ (Variables|Default|GetTotalTime) (Utilities|Time|GetWorldDeltaSeconds))))
      (if (> _output_get (Variables|Default|GetWaitingTimeBetweenPhases))
        (Variables|Default|SetHasWaitedPhase4 true)))))

(event Custom|Phase%203
  (bind _rotator (CallFunction|GetRotationTowardsPlayer))
  (bind _defaultsceneroot (Variables|Default|GetDefaultSceneRoot))
  (bind _returnvalue (Transformation|GetWorldLocation _defaultsceneroot))
  ;[1 1 1] This phase could not be in a function because it has a delay
  ;[1 1 1] Wait 2 sec after phase change
  (if (Variables|Default|GetHasWaitedPhase3)
    (Utilities|FlowControl|Sequence
      (:then_0
        ;[1 1 1] Time attacks
        (if (> (Variables|Default|GetTotalTime) (Variables|Phase3|GetSeconsBetweenAttacksPhase3))
          (Variables|Default|SetTotalTime 0.0)
          ;[1 1 1] Set Vector directions
          (Variables|Phase3|SetAOE_Direction0 (* (Math|Vector|RotateVector "1.000000,0.000000,0.000000" _rotator) 1000))
          (Variables|Phase3|SetAOE_Direction1 (* (Math|Vector|RotateVector "0.866025,0.500000,0.000000" _rotator) 1000))
          (Variables|Phase3|SetAOE_Direction2 (* (Math|Vector|RotateVector "0.866025,-0.500000,0.000000" _rotator) 1000))
          (bind _index (Utilities|ForLoopwithDelay 1 4 0.5)
            (:LoopBody
              ;[1 1 1] Spawn 3 AOE attacks
              (Game|SpawnActorfromClass "/Game/Blueprints/BP_AOE_Attack.BP_AOE_Attack_C" (Math|Conversions|ToTransform(Vector) (+ (* (Variables|Phase3|GetAOE_Direction0) _index) _returnvalue)) "Undefined" 0 0)
              (Game|SpawnActorfromClass "/Game/Blueprints/BP_AOE_Attack.BP_AOE_Attack_C" (Math|Conversions|ToTransform(Vector) (+ (* (Variables|Phase3|GetAOE_Direction1) _index) _returnvalue)) "Undefined" 0 0)
              (Game|SpawnActorfromClass "/Game/Blueprints/BP_AOE_Attack.BP_AOE_Attack_C" (Math|Conversions|ToTransform(Vector) (+ (* (Variables|Phase3|GetAOE_Direction2) _index) _returnvalue)) "Undefined" 0 0)))))
      (:then_1
        ;[1 1 1] Time attacks
        (if (> (Variables|Default|GetTotalTime2) (Variables|Phase3|GetSecondsBetweenAttacksPhase3,2))
          (Variables|Default|SetTotalTime2 0.0)
          ;[1 1 1] Alternate Attack
          (bind _output_get (Variables|Default|SetAttackAlternator (not (Variables|Default|GetAttackAlternator))))
          (if _output_get
            ;[1 1 1] Spawn bouncing bullets
            (for _index_2 (range 0 35)
              (bind _returnvalue_2 (Game|SpawnActorfromClass "/Game/Blueprints/BP_BossProjectile.BP_BossProjectile_C" (Math|Transform|MakeTransform (+ (Transformation|GetActorLocation) "0.000000, 0,100.000000") (Math|Rotator|MakeRotator 0.0 0.0 (Math|Conversions|ToFloat(Integer) (* _index_2 10)))) "Undefined" 0 0))
              (Variables|/Script/Engine.ProjectileMovementComponent|SetProjectileGravityScale (Variables|/Game/Blueprints/BP_BossProjectile.BP_BossProjectile_C|GetProjectileMovement _returnvalue_2) 1.0)
              (Game|Components|ProjectileMovement|SetVelocityinLocalSpace (Variables|/Game/Blueprints/BP_BossProjectile.BP_BossProjectile_C|GetProjectileMovement _returnvalue_2) (Math|Vector|MakeVector (.x (Variables|/Script/Engine.MovementComponent|GetVelocity (Variables|/Game/Blueprints/BP_BossProjectile.BP_BossProjectile_C|GetProjectileMovement _returnvalue_2))) (.y (Variables|/Script/Engine.MovementComponent|GetVelocity (Variables|/Game/Blueprints/BP_BossProjectile.BP_BossProjectile_C|GetProjectileMovement _returnvalue_2))) 1e+03))
              (Variables|/Script/Engine.ProjectileMovementComponent|SetbShouldBounce (Variables|/Game/Blueprints/BP_BossProjectile.BP_BossProjectile_C|GetProjectileMovement _returnvalue_2) true)
              (Collision|SetCollisionResponsetoChannel (Variables|/Game/Blueprints/BP_BossProjectile.BP_BossProjectile_C|GetCollision _returnvalue_2) "ECC_WorldStatic" "ECR_Block"))
            (else
              ;[1 1 1] Spawn 10 bullets in cirlce form
              (for _index_3 (range 0 9)
                (Game|SpawnActorfromClass "/Game/Blueprints/BP_BossProjectile.BP_BossProjectile_C" (Math|Transform|MakeTransform (+ (Transformation|GetActorLocation) "0.000000, 0,100.000000") (Math|Rotator|MakeRotator 0.0 0.0 (* (+ (Math|Conversions|ToFloat(Integer) _index_3) 0.5) 36.0))) "Undefined" 0 0))))
          (Audio|SpawnSoundatLocation "/Game/BossAssets/BallSpawn.BallSpawn" "0, 0,100.000000" "0, 0, 0" 1.0 1.0 0.0 0 0))))
    (else
      (bind _output_get_2 (Variables|Default|SetTotalTime (+ (Variables|Default|GetTotalTime) (Utilities|Time|GetWorldDeltaSeconds))))
      (if (> _output_get_2 (Variables|Default|GetWaitingTimeBetweenPhases))
        (Variables|Default|SetHasWaitedPhase3 true)))))

(event EventBeginPlay)

(event Collision|EventActorBeginOverlap
  (params (OtherActor :type Actor%20Object%20Reference)))

(event EventTick
  (params (DeltaSeconds :type Float%20%28single-precision%29))
  (bind _box (Variables|Default|GetBox))
  (bind _health (Variables|Default|GetHealth))
  (bind _returnvalue (Class|HealthComponent|GetHealthPercentage _health))
  (bind _returnvalue_2 (Transformation|GetWorldLocation _box))
  ;[1 1 1] Phase logic
  (Variables|Phase4|SetTotalTime3 (+ DeltaSeconds (Variables|Phase4|GetTotalTime3)))
  (Variables|Default|SetTotalTime2 (+ DeltaSeconds (Variables|Default|GetTotalTime2)))
  (Variables|Default|SetTotalTime (+ DeltaSeconds (Variables|Default|GetTotalTime)))
  (if (> _returnvalue 0.75)
    (CallFunction|Phase1Attack)
    (Development|PrintString "Phase 1" true true "(R=0.000000,G=0.660000,B=1.000000,A=1.000000)" 0.0)
    ;[1 1 1] Spawn Directed attack that the player has to jump over
    (Utilities|FlowControl|DoOnce false
      (:Completed
        (Audio|PlaySoundatLocation "/Game/BossAssets/Bowser_Laugh.Bowser_Laugh" _returnvalue_2 "0, 0, 0" 1.0 1.0 0.0 0 0 0)))
    (elif (> _returnvalue 0.5)
      (CallFunction|Phase2Attack)
      (Development|PrintString "Phase 2" true true "(R=0.000000,G=0.660000,B=1.000000,A=1.000000)" 0.0)
      (Utilities|FlowControl|DoOnce false
        (:Completed
          (Audio|PlaySoundatLocation "/Game/BossAssets/Bowser_Laugh.Bowser_Laugh" _returnvalue_2 "0, 0, 0" 1.0 1.0 0.0 0 0 0)
          (CallFunction|BetweenPhasesJumpCircle)
          (Variables|Default|SetTotalTime 0.0)
          (Variables|Default|SetTotalTime2 0.0)))
      (elif (> _returnvalue 0.25)
        (CallFunction|Phase3)
        (Development|PrintString "Phase 3" true true "(R=0.000000,G=0.660000,B=1.000000,A=1.000000)" 0.0)
        (Utilities|FlowControl|DoOnce false
          (:Completed
            (Audio|PlaySoundatLocation "/Game/BossAssets/Bowser_Laugh.Bowser_Laugh" _returnvalue_2 "0, 0, 0" 1.0 1.0 0.0 0 0 0)
            (CallFunction|BetweenPhasesJumpCircle)
            (Variables|Default|SetTotalTime 0.0)
            (Variables|Default|SetTotalTime2 0.0)
            (Utilities|FlowControl|Delay 1.2)
            (CallFunction|BetweenPhasesJumpCircle)))
        (elif (> _returnvalue 0.0)
          (CallFunction|Phase4)
          (Development|PrintString "Phase 4" true true "(R=0.000000,G=0.660000,B=1.000000,A=1.000000)" 0.0)
          (Utilities|FlowControl|DoOnce false
            (:Completed
              (Audio|PlaySoundatLocation "/Game/BossAssets/Bowser_Laugh.Bowser_Laugh" _returnvalue_2 "0, 0, 0" 1.0 1.0 0.0 0 0 0)
              (CallFunction|BetweenPhasesJumpCircle)
              (Variables|Default|SetTotalTime 0.0)
              (Variables|Default|SetTotalTime2 0.0)
              (Utilities|FlowControl|Delay 1.2)
              (CallFunction|BetweenPhasesJumpCircle)
              (Utilities|FlowControl|Delay 1.2)
              (CallFunction|BetweenPhasesJumpCircle))))))))

(fn ConstructionScript)

(fn Phase1Attack
  ;[1 1 1] Time attacks
  (if (> (Variables|Default|GetTotalTime) (LocalVariables|GetSeconds%20between%20attacks))
    (Variables|Default|SetTotalTime 0.0)
    ;[1 1 1] Spawn 10 bullets in cirlce form
    (for _index (range 0 9)
      (Game|SpawnActorfromClass "/Game/Blueprints/BP_BossProjectile.BP_BossProjectile_C" (Math|Transform|MakeTransform (+ (Transformation|GetActorLocation) "0.000000, 0,100.000000") (Math|Rotator|MakeRotator 0.0 0.0 (Math|Conversions|ToFloat(Integer) (* _index 36)))) "Undefined" 0 0))
    (Audio|SpawnSoundatLocation "/Game/BossAssets/BallSpawn.BallSpawn" "0, 0,100.000000" "0, 0, 0" 1.0 1.0 0.0 0 0)))

(fn Phase2Attack
  (bind _returnvalue (Game|Player|GetPlayerPawn 0))
  (bind _returnvalue_2 (Transformation|GetActorLocation _returnvalue))
  ;[1 1 1] Wait 2 sec after phase change
  (if (Variables|Default|GetHasWaitedPhase2)
    (Utilities|FlowControl|Sequence
      (:then_0
        ;[1 1 1] Time attacks
        (if (> (Variables|Default|GetTotalTime) (LocalVariables|GetSecondsBetweenAttacks))
          (Variables|Default|SetTotalTime 0.0)
          ;[1 1 1] Alternate Attack
          (bind _output_get (Variables|Default|SetAttackAlternator (not (Variables|Default|GetAttackAlternator))))
          (if _output_get
            ;[1 1 1] Spawn 10 bullets in cirlce form
            (for _index (range 0 9)
              (Game|SpawnActorfromClass "/Game/Blueprints/BP_BossProjectile.BP_BossProjectile_C" (Math|Transform|MakeTransform (+ (Transformation|GetActorLocation) "0.000000, 0,100.000000") (Math|Rotator|MakeRotator 0.0 0.0 (Math|Conversions|ToFloat(Integer) (* _index 36)))) "Undefined" 0 0))
            (else
              ;[1 1 1] Spawn 10 bullets in cirlce form
              (for _index_2 (range 0 9)
                (Game|SpawnActorfromClass "/Game/Blueprints/BP_BossProjectile.BP_BossProjectile_C" (Math|Transform|MakeTransform (+ (Transformation|GetActorLocation) "0.000000, 0,100.000000") (Math|Rotator|MakeRotator 0.0 0.0 (* (+ (Math|Conversions|ToFloat(Integer) _index_2) 0.5) 36.0))) "Undefined" 0 0))))
          (Audio|SpawnSoundatLocation "/Game/BossAssets/BallSpawn.BallSpawn" "0, 0,100.000000" "0, 0, 0" 1.0 1.0 0.0 0 0)))
      (:then_1
        ;[1 1 1] Time attacks
        (if (> (Variables|Default|GetTotalTime2) (LocalVariables|GetSecondsBetweenAttacks2))
          (Variables|Default|SetTotalTime2 0.0)
          (bind _returnvalue_3 (Game|SpawnActorfromClass "/Game/Blueprints/BP_BossProjectile.BP_BossProjectile_C" (Math|Transform|MakeTransform (+ (Transformation|GetActorLocation) "0.000000, 0,100.000000") (Math|Rotator|FindLookatRotation (Math|Vector|MakeVector -1.0 0.0 0.0) (Math|Vector|Normalize (- _returnvalue_2 (Math|Vector|MakeVector 0.0 0.0 (.Z (Math|Vector|BreakVector _returnvalue_2))))))) "Undefined" 0 0))
          ;[1 1 1] Make it faster than normal bullets
          (Game|Components|ProjectileMovement|SetVelocityinLocalSpace (Variables|/Game/Blueprints/BP_BossProjectile.BP_BossProjectile_C|GetProjectileMovement _returnvalue_3) (* (Variables|/Script/Engine.MovementComponent|GetVelocity (Variables|/Game/Blueprints/BP_BossProjectile.BP_BossProjectile_C|GetProjectileMovement _returnvalue_3)) 1.6)))))
    (else
      (bind _output_get_2 (Variables|Default|SetTotalTime (+ (Variables|Default|GetTotalTime) (Utilities|Time|GetWorldDeltaSeconds))))
      (if (> _output_get_2 (Variables|Default|GetWaitingTimeBetweenPhases))
        (Variables|Default|SetHasWaitedPhase2 true)))))

(fn BetweenPhasesJumpCircle
  ;[1 1 1] Spawn 100 bullets in cirlce form
  (for _index (range -15 15)
    (Game|SpawnActorfromClass "/Game/Blueprints/BP_BossProjectile.BP_BossProjectile_C" (Math|Transform|MakeTransform (+ (Transformation|GetActorLocation) "0.000000, 0,100.000000") (Math|Conversions|RotationFromXVector (Math|Vector|RotateVector (Math|Vector|MakeVector (Math|Trig|Cos(Degrees) (* _index 2.3)) (Math|Trig|Sin(Degrees) (* _index 2.3)) 0.0) (CallFunction|GetRotationTowardsPlayer)))) "Undefined" 0 0))
  (Audio|SpawnSoundatLocation "/Game/BossAssets/BallSpawn.BallSpawn" "0, 0,100.000000" "0, 0, 0" 1.0 1.0 0.0 0 0))

(fn GetRotationTowardsPlayer
  (bind _returnvalue (Game|Player|GetPlayerPawn 0))
  (bind _returnvalue_2 (Transformation|GetActorLocation _returnvalue))
  (return (Math|Rotator|FindLookatRotation (Math|Vector|MakeVector 0.0 0.0 0.0) (- _returnvalue_2 (Math|Vector|MakeVector 0.0 0.0 (.Z (Math|Vector|BreakVector _returnvalue_2)))))))