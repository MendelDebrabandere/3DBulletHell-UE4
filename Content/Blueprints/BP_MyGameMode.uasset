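; Game mode that resets the boss fight through a RespawnPlayer event.
; It destroys any existing BP_Boss and spawns a fresh one at a fixed location, then spawns the default pawn at a player start and has the first player controller possess it.
; After a brief delay, it clears leftover player projectiles, boss projectiles and AOE attacks by destroying every actor of those classes.
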(event Custom|RespawnPlayer
  (bind _returnvalue (Game|GetPlayerController 0))
  ;[1 1 1] Respawn Boss
  (bind _outactors (Actor|GetAllActorsOfClass "/Game/Blueprints/BP_Boss.BP_Boss_C"))
  (for _array_element _outactors
    (Actor|DestroyActor _array_element))
  (Game|SpawnActorfromClass "/Game/Blueprints/BP_Boss.BP_Boss_C" (Math|Conversions|ToTransform(Vector) (Math|Vector|MakeVector 0.0 0.0 5e+01)) "Undefined" 0 0)
  ;[1 1 1] Respawn Player
  (bind _returnvalue_2 (Game|SpawnActorfromClass (Variables|Default|GetDefaultPawnClass) (Transformation|GetActorTransform (Class|GameModeBase|FindPlayerStart _returnvalue)) "Undefined" 0 0))
  (Pawn|Possess _returnvalue _returnvalue_2)
  (Utilities|FlowControl|Delay 0.01)
  ;[1 1 1] Destroy player projectiles
  (bind _outactors_2 (Actor|GetAllActorsOfClass "/Game/Blueprints/BP_BaseProjectile.BP_BaseProjectile_C"))
  (for _array_element_2 _outactors_2
    (Actor|DestroyActor _array_element_2))
  ;[1 1 1] Destroy boss projectiles
  (bind _outactors_3 (Actor|GetAllActorsOfClass "/Game/Blueprints/BP_BossProjectile.BP_BossProjectile_C"))
  (for _array_element_3 _outactors_3
    (Actor|DestroyActor _array_element_3))
  ;[1 1 1] Destroy AOE attacks
  (bind _outactors_4 (Actor|GetAllActorsOfClass "/Game/Blueprints/BP_AOE_Attack.BP_AOE_Attack_C"))
  (for _array_element_4 _outactors_4
    (Actor|DestroyActor _array_element_4)))

(event EventBeginPlay)

(event EventTick
  (params (DeltaSeconds :type Float%20%28single-precision%29)))

(fn ConstructionScript)