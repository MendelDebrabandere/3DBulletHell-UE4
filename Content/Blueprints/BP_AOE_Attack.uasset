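; Telegraphed area-of-effect attack actor that warns with circle decals, then explodes and damages the player if within range.
; BeginPlay sets the tuning values, shows the outer circle, and activates the inner circle after a fraction of the lifespan.
; Tick counts down and scales the inner decal on Y and Z as a progress indicator.
; At expiry it spawns explosion effects, distance-checks player 0 for Health damage, and destroys itself.
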(event Custom|DealDamage
  (bind _returnvalue (Game|GetPlayerCharacter 0))
  ;[1 1 1] Deal damage to player if is in range
  (if (< (Math|Vector|Distance(Vector) (Transformation|GetActorLocation _returnvalue) (Transformation|GetWorldLocation (Variables|Default|GetDefaultSceneRoot))) (Variables|Settings|GetDamageRadius))
    (bind _asbp_player_character (Utilities|Casting|CastToBP_PlayerCharacter _returnvalue))
    (Class|HealthComponent|DoDamage (Variables|/Game/Blueprints/BP_BaseCharacter.BP_BaseCharacter_C|GetHealth _asbp_player_character) (Variables|Settings|GetDamageAmount))))

(event EventBeginPlay
  ;[1 1 1] Setting up variables
  (Variables|Settings|SetLifeSpan 3.0)
  (Variables|Settings|SetDamageAmount 15.0)
  (Variables|Settings|SetDamageRadius 512.0)
  (Variables|Settings|SetWaitingBefoirInnerCircleScalar 3.0)
  ;[1 1 1] Activate decals
  (Components|Activation|Activate (Variables|Default|GetOuterCircle) false)
  (Utilities|FlowControl|Delay (/ (Variables|Settings|GetLifeSpan) (Variables|Settings|GetWaitingBefoirInnerCircleScalar)))
  (Variables|Settings|SetLifeSpan (- (Variables|Settings|GetLifeSpan) (/ (Variables|Settings|GetLifeSpan) (Variables|Settings|GetWaitingBefoirInnerCircleScalar))))
  (Components|Activation|Activate (Variables|Default|GetInnerCircle) false)
  (Variables|Settings|SetTempLifeSpanVariable (Variables|Settings|GetLifeSpan)))

(event Collision|EventActorBeginOverlap
  (params (OtherActor :type Actor%20Object%20Reference)))

(event EventTick
  (params (DeltaSeconds :type Float%20%28single-precision%29))
  (bind _innercircle (Variables|Default|GetInnerCircle))
  (bind _defaultsceneroot (Variables|Default|GetDefaultSceneRoot))
  (bind _returnvalue (Transformation|GetWorldLocation _defaultsceneroot))
  ;[1 1 1] Check if it reached max size
  (if (> (Variables|Settings|GetLifeSpan) 0.0)
    ;[1 1 1] Increase size
    (bind _output_get (Variables|Settings|SetLifeSpan (- (Variables|Settings|GetLifeSpan) (Utilities|Time|GetWorldDeltaSeconds))))
    (Transformation|SetWorldScale3D _innercircle (Math|Vector|MakeVector (.x (Transformation|GetWorldScale _innercircle)) (/ (- (Variables|Settings|GetTempLifeSpanVariable) _output_get) (Variables|Settings|GetTempLifeSpanVariable)) (/ (- (Variables|Settings|GetTempLifeSpanVariable) _output_get) (Variables|Settings|GetTempLifeSpanVariable))))
    (else
      ;[1 1 1] Explode
      (Effects|SpawnEmitteratLocation "/Game/StarterContent/Particles/P_Explosion.P_Explosion" _returnvalue "0, 0, 0" "5.000000,5.000000,5.000000")
      (Audio|SpawnSoundatLocation "/Game/StarterContent/Audio/Explosion02.Explosion02" _returnvalue "0, 0, 0" 1.0 1.0 0.0 0 0)
      (CallFunction|DealDamage)
      (Actor|DestroyActor))))

(event EventDestroyed)

(fn ConstructionScript)