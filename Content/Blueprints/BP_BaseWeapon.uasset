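; BP_BaseWeapon is a base weapon Blueprint that handles automatic primary fire.
; FirePrimary takes a start flag, firing one shot immediately and starting a looping timer at the PrimaryFireRate interval in shots per second.
; A DoOnce gate blocks repeated starts until a stop clears the timer by function name and resets the gate.
; Each shot spawns the PrimaryProjectile class and a sound at the FireSocket.
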(event Custom|FirePrimary
  (params (IsStart :type Boolean))
  (if IsStart
    (Utilities|FlowControl|DoOnce false :!label _label
      (:Completed
        (CallFunction|SpawnPrimaryProjectile)
        (Utilities|Time|SetTimerbyEvent (delegate Custom|SpawnPrimaryProjectile) (/ 1.0 (Variables|Default|GetPrimaryFireRate)) true)))
    (else
      (Utilities|Time|ClearTimerbyFunctionName 0 "SpawnPrimaryProjectile")
      (goto _label Reset))))

(event Custom|SpawnPrimaryProjectile
  (Game|SpawnActorfromClass (Variables|Default|GetPrimaryProjectile) (Transformation|GetWorldTransform (Variables|Default|GetFireSocket)) "Undefined" 0 0)
  (Audio|SpawnSoundatLocation "/Game/PlayerAssets/FPWeapon/FREE_Sci-Fi_Weapons_Sound_Effects.FREE_Sci-Fi_Weapons_Sound_Effects" (Transformation|GetWorldLocation (Variables|Default|GetFireSocket)) "0, 0, 0" 1.0 1.0 0.0 0 0))

(event EventBeginPlay)

(event Collision|EventActorBeginOverlap
  (params (OtherActor :type Actor%20Object%20Reference)))

(event EventTick
  (params (DeltaSeconds :type Float%20%28single-precision%29)))

(fn ConstructionScript)